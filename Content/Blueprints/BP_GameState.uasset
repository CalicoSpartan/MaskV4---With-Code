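; BP_GameState is a game state Blueprint that drives two HUD elements: a kill feed and a game-over screen.
; CallHUDUpdate creates a KillFeedEntry widget from KillFeedMessage and adds it to the UI reference's vertical box, printing a warning if that reference is invalid.
; CallHUDGameOver creates a GameOverUI widget, fills its winning-team text from WinningMessage, and adds it to the viewport.
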(event `self.ReceiveBeginPlay`)

(event `AddKillFeedMessage`
  ;[1 1 1] KillFeedMessages
  (`/Engine/EditorBlueprintResources/StandardMacros.IsValid` (`self.UI`)
    (:`Is Valid`
      (bind _returnvalue (`|CreateWidget` "/Game/UI/KillFeedEntry.KillFeedEntry_C" null (`KismetTextLibrary.Conv_StringToText` (`self.KillFeedMessage`))))
      (bind _output_get (set `self.Entry` _returnvalue))
      (`VerticalBox.AddChildToVerticalBox` (`/Game/UI/InGameUI.VerticalBox_0` (`self.UI`)) _output_get))
    (:`Is Not Valid`
      (`KismetSystemLibrary.PrintString` "GameState has no UI reference" true true (struct :`R` 0.090628 :`G` 0.28 :`B` 0.073843 :`A` 1.0) 40.0))))

(event `self.CallHUDUpdate`
  ;[1 1 1] KillFeedMessages
  (`self.AddKillFeedMessage`))

(event `AddGameOverUI`
  (bind _gameoverui (`self.GameOverUI`))
  ;[1 1 1] gameoverUI
  (bind _returnvalue (`|CreateWidget` "/Game/UI/GameOverUI.GameOverUI_C"))
  (set `self.GameOverUI` _returnvalue)
  (`TextBlock.SetText` (`/Game/UI/GameOverUI.WinningTeamText` _gameoverui) (`KismetTextLibrary.Conv_StringToText` (`self.WinningMessage`)))
  (`UserWidget.AddToViewport` _gameoverui 4))

(event `self.CallHUDGameOver`
  ;[1 1 1] gameoverUI
  (`self.AddGameOverUI`))

(fn `UserConstructionScript`)
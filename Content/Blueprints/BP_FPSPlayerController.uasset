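; Player controller for a team FPS that builds and updates the in-game HUD, team score bars and scoreboard.
; UIBlueprint-suffixed events trigger widget creation and refresh, and the HUD is also stored on BP_GameState.
; The scoreboard creates one row per player state in two team boxes, and holding Tab shows it.
; Refreshes fill rows by index from GameState's team order arrays when lengths match, highlighting the controller's own player.
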(event `self.UpdateScoreUIBlueprint`
  ;[1 1 1] ScoreUI
  (`self.UpdateScore`))

(event `UpdateScore`
  (bind _scoreui (`self.ScoreUI`))
  ;[1 1 1] ScoreUI
  (`/Engine/EditorBlueprintResources/StandardMacros.IsValid` (`self.ScoreUI`)
    (:`Is Valid`
      (`ProgressBar.SetPercent` (`/Game/UI/ScoreUI.MyScore` _scoreui) (`self.TeamScorePercent`))
      (`ProgressBar.SetPercent` (`/Game/UI/ScoreUI.EnemyScore` _scoreui) (`self.RivalScorePercent`)))))

(event `self.TriggerAddAliveUIBlueprint`
  ;[1 1 1] GameUI
  (`self.AddGameUIToClient`))

(event `Key|Tab`
  (params (Key :type "Key Structure" :default "AnyKey"))
  (:`Pressed`
    (`self.ShowScoreBoard`))
  (:`Released`
    (`self.RemoveScoreBoard`)))

(event `AddGameUIToClient`
  ;[1 1 1] GameUI
  (`/Engine/EditorBlueprintResources/StandardMacros.IsValid` (`self.InGameUI`)
    (:`Is Not Valid`
      (bind _returnvalue (`|CreateWidget` "/Game/UI/InGameUI.InGameUI_C"))
      (bind _output_get (set `self.InGameUI` _returnvalue))
      (bind _asbp_game_state (cast `/Game/Blueprints/BP_GameState` (`GameplayStatics.GetGameState`)))
      (set `/Game/Blueprints/BP_GameState.UI` _returnvalue _asbp_game_state)
      (`UserWidget.AddToViewport` _output_get 0)
      (bind _returnvalue_2 (`|CreateWidget` "/Game/UI/ScoreUI.ScoreUI_C"))
      (bind _output_get_2 (set `self.ScoreUI` _returnvalue_2))
      (`UserWidget.AddToViewport` _output_get_2 1))))

(event `ShowScoreBoard`
  (bind _scoreboardui (`self.ScoreBoardUI`))
  (`/Engine/EditorBlueprintResources/StandardMacros.IsValid` _scoreboardui
    (:`Is Valid`
      (`Widget.SetVisibility` _scoreboardui "Visible"))))

(event `RemoveScoreBoard`
  (bind _scoreboardui (`self.ScoreBoardUI`))
  (`/Engine/EditorBlueprintResources/StandardMacros.IsValid` _scoreboardui
    (:`Is Valid`
      (`Widget.SetVisibility` _scoreboardui "Hidden"))))

(event `self.AddScoreBoardUIBlueprint`
  ;[1 1 1] base scoreboard
  (`self.AddScoreBoardToClient`))

(event `AddScoreBoardToClient`
  (bind _scoreboardui (`self.ScoreBoardUI`))
  ;[1 1 1] base scoreboard
  (`/Engine/EditorBlueprintResources/StandardMacros.IsValid` (`self.ScoreBoardUI`)
    (:`Is Not Valid`
      (bind _returnvalue (`|CreateWidget` "/Game/UI/ScoreBoardUI.ScoreBoardUI_C"))
      (set `self.ScoreBoardUI` _returnvalue)
      (bind _returnvalue_2 (`|CreateWidget` "/Game/UI/TeamScoreBoard.TeamScoreBoard_C"))
      (bind _output_get (set `self.Team1Stats` _returnvalue_2))
      (`TextBlock.SetText` (`/Game/UI/TeamScoreBoard.TeamNameHere` _output_get) "Team1")
      (`VerticalBox.AddChildToVerticalBox` (`/Game/UI/ScoreBoardUI.VerticalScoreBox` (`self.ScoreBoardUI`)) _output_get)
      (bind _returnvalue_3 (`|CreateWidget` "/Game/UI/TeamScoreBoard.TeamScoreBoard_C"))
      (bind _output_get_2 (set `self.Team2Stats` _returnvalue_3))
      (`TextBlock.SetText` (`/Game/UI/TeamScoreBoard.TeamNameHere` _output_get_2) "Team2")
      (`VerticalBox.AddChildToVerticalBox` (`/Game/UI/ScoreBoardUI.VerticalScoreBox` (`self.ScoreBoardUI`)) _output_get_2)
      (bind _asbp_game_state (cast `/Game/Blueprints/BP_GameState` (`GameplayStatics.GetGameState`)))
      (for _ (`FPSGameState.Team1PlayerStates` _asbp_game_state)
        (bind _returnvalue_4 (`|CreateWidget` "/Game/UI/PlayerStats.PlayerStats_C"))
        (`UserWidget.SetColorAndOpacity` _returnvalue_4 (struct :`G` 0.024323 :`B` 0.625 :`A` 1.0))
        (`VerticalBox.AddChildToVerticalBox` (`/Game/UI/TeamScoreBoard.AddTeamsToThisBox` (`self.Team1Stats`)) _returnvalue_4))
      (bind _asbp_game_state_2 (cast `/Game/Blueprints/BP_GameState` (`GameplayStatics.GetGameState`)))
      (for _ (`FPSGameState.Team2PlayerStates` _asbp_game_state_2)
        (bind _returnvalue_5 (`|CreateWidget` "/Game/UI/PlayerStats.PlayerStats_C"))
        (`UserWidget.SetColorAndOpacity` _returnvalue_5 (struct :`R` 0.665 :`B` 0.018856 :`A` 1.0))
        (`VerticalBox.AddChildToVerticalBox` (`/Game/UI/TeamScoreBoard.AddTeamsToThisBox` (`self.Team2Stats`)) _returnvalue_5))
      (`Widget.SetVisibility` _scoreboardui "Hidden")
      (`UserWidget.AddToViewport` _scoreboardui 5)
      (set `self.CanUpdateScoreBoard` true))))

(event `UpdatePlayerStats`
  (bind _team1stats (`self.Team1Stats`))
  (bind _team2stats (`self.Team2Stats`))
  ;[1 1 1] UpdateScoreBoard
  (bind _asbp_game_state (cast `/Game/Blueprints/BP_GameState` (`GameplayStatics.GetGameState`)))
  (if (== (`KismetArrayLibrary.Array_Length` (`FPSGameState.Team2PlayerOrder` _asbp_game_state)) (`KismetArrayLibrary.Array_Length` (`FPSGameState.Team2PlayerStates` _asbp_game_state)))
    (bind _team1playerorder (`FPSGameState.Team1PlayerOrder` _asbp_game_state))
    (if (== (`KismetArrayLibrary.Array_Length` _team1playerorder) (`KismetArrayLibrary.Array_Length` (`FPSGameState.Team1PlayerStates` _asbp_game_state)))
      (for (_array_element _array_index) _team1playerorder
        (if (`KismetArrayLibrary.Array_IsValidIndex` _team1playerorder _array_index)
          (bind _asbp_fpsplayer_state (cast `/Game/Blueprints/BP_FPSPlayerState` _array_element)
            (:`then`
              (bind _returnvalue (`FPSPlayerState.GetScore` _asbp_fpsplayer_state))
              (bind _returnvalue_2 (`FPSPlayerState.GetKills` _asbp_fpsplayer_state))
              (bind _returnvalue_3 (`FPSPlayerState.GetDeaths` _asbp_fpsplayer_state))
              (bind _returnvalue_4 (`FPSPlayerState.GetAssists` _asbp_fpsplayer_state))
              (`/Engine/EditorBlueprintResources/StandardMacros.IsValid` _team1stats
                (:`Is Valid`
                  (bind _returnvalue_5 (`PanelWidget.GetChildAt` (`/Game/UI/TeamScoreBoard.AddTeamsToThisBox` _team1stats) _array_index))
                  (`/Engine/EditorBlueprintResources/StandardMacros.IsValid` _returnvalue_5
                    (:`Is Valid`
                      (bind _asplayer_stats (cast `/Game/UI/PlayerStats` _returnvalue_5))
                      (`TextBlock.SetText` (`/Game/UI/PlayerStats.AssistsHere` _asplayer_stats) (`KismetTextLibrary.Conv_IntToText` _returnvalue_4))
                      (`TextBlock.SetText` (`/Game/UI/PlayerStats.ScoreHere` _asplayer_stats) (`KismetTextLibrary.Conv_IntToText` _returnvalue))
                      (`TextBlock.SetText` (`/Game/UI/PlayerStats.KillsHere` _asplayer_stats) (`KismetTextLibrary.Conv_IntToText` _returnvalue_2))
                      (`TextBlock.SetText` (`/Game/UI/PlayerStats.DeathsHere` _asplayer_stats) (`KismetTextLibrary.Conv_IntToText` _returnvalue_3))
                      (`TextBlock.SetText` (`/Game/UI/PlayerStats.PlayerNameHere` _asplayer_stats) (`KismetTextLibrary.Conv_StringToText` (`FPSPlayerState.UserName` _asbp_fpsplayer_state)))
                      (bind _asbp_fpsplayer_state_2 (cast `/Game/Blueprints/BP_FPSPlayerState` (`self.PlayerState`)))
                      (if (== _asbp_fpsplayer_state _asbp_fpsplayer_state_2)
                        (`UserWidget.SetColorAndOpacity` _asplayer_stats (struct :`R` 0.871367 :`G` 0.783538 :`B` 0.056128 :`A` 1.0))
                        (else
                          (`UserWidget.SetColorAndOpacity` _asplayer_stats (struct :`G` 0.024158 :`B` 0.623961 :`A` 1.0)))))))))
            (:`CastFailed`
              (`KismetSystemLibrary.PrintString` "bad" true true (struct :`G` 1.0 :`B` 0.447663 :`A` 1.0) 200.0)))
          (else
            (`KismetSystemLibrary.PrintString` "not valid index" true true (struct :`G` 0.66 :`B` 1.0 :`A` 1.0) 200.0))))
      (bind _team2playerorder (`FPSGameState.Team2PlayerOrder` _asbp_game_state))
      (for (_array_element_2 _array_index_2) _team2playerorder
        (if (`KismetArrayLibrary.Array_IsValidIndex` _team2playerorder _array_index_2)
          (bind _asbp_fpsplayer_state_3 (cast `/Game/Blueprints/BP_FPSPlayerState` _array_element_2))
          (bind _returnvalue_6 (`FPSPlayerState.GetScore` _asbp_fpsplayer_state_3))
          (bind _returnvalue_7 (`FPSPlayerState.GetKills` _asbp_fpsplayer_state_3))
          (bind _returnvalue_8 (`FPSPlayerState.GetDeaths` _asbp_fpsplayer_state_3))
          (bind _returnvalue_9 (`FPSPlayerState.GetAssists` _asbp_fpsplayer_state_3))
          (bind _returnvalue_10 (`FPSPlayerState.GetUserName` _asbp_fpsplayer_state_3))
          (`/Engine/EditorBlueprintResources/StandardMacros.IsValid` _team2stats
            (:`Is Valid`
              (bind _returnvalue_11 (`PanelWidget.GetChildAt` (`/Game/UI/TeamScoreBoard.AddTeamsToThisBox` _team2stats) _array_index_2))
              (`/Engine/EditorBlueprintResources/StandardMacros.IsValid` _returnvalue_11
                (:`Is Valid`
                  (bind _asplayer_stats_2 (cast `/Game/UI/PlayerStats` _returnvalue_11))
                  (`TextBlock.SetText` (`/Game/UI/PlayerStats.AssistsHere` _asplayer_stats_2) (`KismetTextLibrary.Conv_IntToText` _returnvalue_9))
                  (`TextBlock.SetText` (`/Game/UI/PlayerStats.ScoreHere` _asplayer_stats_2) (`KismetTextLibrary.Conv_IntToText` _returnvalue_6))
                  (`TextBlock.SetText` (`/Game/UI/PlayerStats.KillsHere` _asplayer_stats_2) (`KismetTextLibrary.Conv_IntToText` _returnvalue_7))
                  (`TextBlock.SetText` (`/Game/UI/PlayerStats.DeathsHere` _asplayer_stats_2) (`KismetTextLibrary.Conv_IntToText` _returnvalue_8))
                  (`TextBlock.SetText` (`/Game/UI/PlayerStats.PlayerNameHere` _asplayer_stats_2) (`KismetTextLibrary.Conv_StringToText` _returnvalue_10))
                  (bind _asbp_fpsplayer_state_4 (cast `/Game/Blueprints/BP_FPSPlayerState` (`self.PlayerState`)))
                  (if (== _asbp_fpsplayer_state_4 _asbp_fpsplayer_state_3)
                    (`UserWidget.SetColorAndOpacity` _asplayer_stats_2 (struct :`R` 0.871367 :`G` 0.783538 :`B` 0.056128 :`A` 1.0))
                    (else
                      (`UserWidget.SetColorAndOpacity` _asplayer_stats_2 (struct :`R` 0.665387 :`B` 0.0185 :`A` 1.0))))))))
          (else
            (`KismetSystemLibrary.PrintString` "not valid index" true true (struct :`G` 0.66 :`B` 1.0 :`A` 1.0) 200.0)))))))

(event `self.UpdateScoreBoardUIBlueprint`
  ;[1 1 1] UpdateScoreBoard
  (`self.UpdatePlayerStats`))

(fn `UserConstructionScript`)